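; Radio prop that plays a broadcast sound and switches its three display lights.
; BeginPlay toggles the lights' visibility and caches the broadcast's duration, which is not read elsewhere in the file.
; PlayRadioBroadCast toggles the lights again, then plays the sound attached to the Scene component with configurable volume, pitch and start time, fading it in.
; Nothing in this Blueprint calls PlayRadioBroadCast.
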(event EventBeginPlay
  (Rendering|ToggleVisibility (Variables|Default|GetRadioDisplayLight02) false)
  (Variables|Default|SetBroadcastDuration (Variables|/Script/Engine.SoundBase|GetDuration (Variables|Default|GetRadioBroadcast))))

(event EventActorBeginOverlap
  (params (OtherActor :type Actor%20Object%20Reference)))

(fn ConstructionScript)

(fn PlayRadioBroadCast
  (CallFunction|ToggleLightson)
  (bind _returnvalue (Class|GameplayStatics|PlaySoundAttached (Variables|Default|GetRadioBroadcast) (Variables|Default|GetScene) "None" (Transformation|GetActorLocation) "KeepRelativeOffset" false (Variables|Default|GetVolumeMultiplier) (Variables|Default|GetPitchMiltiplier) (Variables|Default|GetStartTime)))
  (Audio|Components|Audio|FadeIn _returnvalue 5.0 1.0 0.0 :!class /Script/Engine.AudioComponent))

(fn ToggleLightson
  (Rendering|ToggleVisibility (Variables|Default|GetRadioDisplayLight01) false))